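; Light shaft VFX actor that scatters instanced SM_LightShaft meshes across a rectangular window area aligned to its rotation.
; SetupLightShaft runs on construction and again on BeginPlay, drawing a debug box of the window and adding randomly placed instances without clearing.
; Instance count scales with NumberLightShaft and window size, while ShaftScale sets their X scale.
; Shaft width and emissive-boosted color reach the material through custom primitive data.
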(event Custom|SetupLightShaft
  (bind _instancedstaticmesh (Variables|Default|GetInstancedStaticMesh))
  (bind _boostemissive (Variables|Default|GetBoostEmissive))
  (bind _instancedstaticmesh_2 (Variables|Default|GetInstancedStaticMesh))
  (bind _lightshaftcolor (Variables|Default|GetLightShaftColor))
  (bind _returnvalue (Math|Conversions|ToLinearColor(Color) _lightshaftcolor))
  (Utilities|FlowControl|Sequence
    (:then_0
      ;[0.1042 0.1042 0.1042] Debug rect
      (Rendering|Debug|DrawDebugBox (+ (Transformation|GetActorLocation) (Math|Vector|RotateVector (Math|Vector|MakeVector 0.0 0.0 (/ (.z (Variables|SetUp|GetWindowHeight)) 2.0)) (Transformation|GetActorRotation))) (Math|Vector|MakeVector 0.0 (.y (Variables|SetUp|GetWindowWidth)) (/ (.z (Variables|SetUp|GetWindowHeight)) 2.0)) "(R=1.000000,G=0.000000,B=0.000000,A=1.000000)" (Transformation|GetActorRotation) 0.0 5.0)
      (Variables|SetUp|SetWindowWidth (Math|Vector|MakeVector 0.0 (.y (Variables|SetUp|GetWindowWidth)) (/ (.z (Variables|SetUp|GetWindowHeight)) 2.0)))
      (Variables|SetUp|SetWindowHeight (Math|Vector|MakeVector 0.0 0.0 (.z (Variables|SetUp|GetWindowHeight))))
      (Variables|SetUp|SetShaftScale (Math|Vector|MakeVector (.x (Variables|SetUp|GetShaftScale)) 0.0 (/ (.z (Variables|SetUp|GetWindowHeight)) 2.0))))
    (:then_1
      ;[0.05445 0.05631 0.166] Istance Thcken mesh
      (if (not (== (Variables|Default|GetNumberLightShaft) 0))
        (Components|StaticMesh|SetStaticMesh _instancedstaticmesh_2 "/Game/VFX/LightShaft/StaticMesh/SM_LightShaft.SM_LightShaft")
        (Class|PrimitiveComponent|SetCullDistance _instancedstaticmesh_2 (Variables|Default|GetCull%20Distance))
        (Rendering|SetCastShadow _instancedstaticmesh false)
        (Rendering|Material|SetCustomPrimitiveDataFloat _instancedstaticmesh 0 (Variables|Default|GetWitdhShaft))
        (Rendering|Material|SetCustomPrimitiveDataVector4 _instancedstaticmesh 1 (Math|Vector4|MakeVector4 (* (.r _returnvalue) _boostemissive) (* (.g _returnvalue) _boostemissive) (* (.b _returnvalue) _boostemissive) (.a _returnvalue)))
        (for _index (range 0 (* (- (Variables|Default|GetNumberLightShaft) 1) (Math|Float|Ceil (* (.y (/ (Math|Vector|MakeVector 0.0 (Math|Vector|VectorLength (Variables|SetUp|GetWindowWidth)) (.z (Variables|SetUp|GetWindowHeight))) "1.000000,100.000000,150.000000")) (.z (/ (Math|Vector|MakeVector 0.0 (Math|Vector|VectorLength (Variables|SetUp|GetWindowWidth)) (.z (Variables|SetUp|GetWindowHeight))) "1.000000,100.000000,150.000000"))))))
          (Components|InstancedStaticMesh|AddInstance (Variables|Default|GetInstancedStaticMesh) (Math|Transform|MakeTransform (+ (Transformation|GetActorLocation) (Math|Vector|RotateVector (Math|Random|RandomPointinBoundingBox (Math|Vector|MakeVector 0.0 0.0 (/ (.z (Variables|SetUp|GetWindowHeight)) 2.0)) (Math|Vector|MakeVector 0.0 (.y (Variables|SetUp|GetWindowWidth)) (/ (.z (Variables|SetUp|GetWindowHeight)) 2.0))) (Transformation|GetActorRotation))) (Transformation|GetActorRotation) (Math|Vector|MakeVector (/ (.x (Variables|SetUp|GetShaftScale)) 24.0) 1.0 1.0)) true))))))

(event EventBeginPlay
  (CallFunction|SetupLightShaft))

(event Collision|EventActorBeginOverlap
  (params (OtherActor :type Actor%20Object%20Reference)))

(event EventTick
  (params (DeltaSeconds :type Float%20%28single-precision%29)))

(fn ConstructionScript
  (CallFunction|SetupLightShaft))