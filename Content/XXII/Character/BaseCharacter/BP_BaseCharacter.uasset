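; Base player character with camera-relative movement, dash, slash queueing and a zoomable spring-arm camera.
; BeginPlay restores a non-default saved transform and stats from the GameInstance's selected save.
; Mouse wheel sets a clamped zoom multiplier; Tick interpolates arm length and updates depth-of-field settings to match, leaving the older Zoom timeline path disconnected.
; Stat interface calls forward to StatComponent, and movement input is ignored during the combo montage.
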(event Input|EnhancedActionEvents|EnhancedInputActionIA_Move
  (params (ActionValue :type Vector%202D%20Structure) (ElapsedSeconds :type Float%20%28double-precision%29) (TriggeredSeconds :type Float%20%28double-precision%29) (InputAction :type Input%20Action%20Object%20Reference :default "/Game/Input/Actions/IA_Move.IA_Move"))
  (bind _camera (Variables|Default|GetCamera))
  (bind _returnvalue (Transformation|GetWorldRotation _camera))
  (if (not (Animation|Montage|MontageIsPlaying (Components|SkeletalMesh|GetAnimInstance (Variables|Character|GetMesh)) "/Game/XXII/Anims/ComboMontage.ComboMontage"))
    (Pawn|Input|AddMovementInput (Math|Vector|GetForwardVector (Math|Rotator|MakeRotator (.roll _returnvalue) 0.0 (.yaw _returnvalue))) (.y (Input|EnhancedActionValues|GetIA_Move)) false)
    (Pawn|Input|AddMovementInput (Math|Vector|GetRightVector (Math|Rotator|MakeRotator 0.0 0.0 (.yaw (Transformation|GetWorldRotation (Variables|Default|GetCamera))))) (.x (Input|EnhancedActionValues|GetIA_Move)) false)))

(event Input|EnhancedActionEvents|EnhancedInputActionIA_Slash
  (params (ActionValue :type Boolean) (ElapsedSeconds :type Float%20%28double-precision%29) (TriggeredSeconds :type Float%20%28double-precision%29) (InputAction :type Input%20Action%20Object%20Reference :default "/Game/Input/Actions/IA_Slash.IA_Slash"))
  (Variables|Default|SetAttackQueued ActionValue))

(event Input|EnhancedActionEvents|EnhancedInputActionIA_MouseLook
  (params (ActionValue :type Vector%202D%20Structure) (ElapsedSeconds :type Float%20%28double-precision%29) (TriggeredSeconds :type Float%20%28double-precision%29) (InputAction :type Input%20Action%20Object%20Reference :default "/Game/Input/Actions/IA_MouseLook.IA_MouseLook"))
  (Pawn|Input|AddControllerYawInput (.x ActionValue)))

(event Input|EnhancedActionEvents|EnhancedInputActionIA_Dash
  (params (ActionValue :type Boolean) (ElapsedSeconds :type Float%20%28double-precision%29) (TriggeredSeconds :type Float%20%28double-precision%29) (InputAction :type Input%20Action%20Object%20Reference :default "/Game/Variant_Platforming/Input/Actions/IA_Dash.IA_Dash"))
  (Class|XXIICharacter|DoDash))

(event EventBeginPlay
  (bind (_fstop _sensorwidth) (Utilities|GetZoomPPSettings))
  (|CallParentFunction)
  (CallFunction|SetPlayerSaveInformation)
  (bind _output_get (Variables|/Script/Engine.SpringArmComponent|SetTargetArmLength (Variables|Default|GetSpringArm) (* (Variables|Zoom|GetZoomMultiplier) (Variables|Zoom|GetZoomStep))))
  (Utilities|Struct|SetmembersinPostProcessSettings (Variables|/Script/Engine.CameraComponent|GetPostProcessSettings (Variables|Default|GetCamera)) _fstop _sensorwidth _output_get))

(event EventTick
  (params (DeltaSeconds :type Float%20%28single-precision%29))
  (bind (_fstop _sensorwidth) (Utilities|GetZoomPPSettings))
  (Utilities|Struct|SetmembersinPostProcessSettings (Variables|/Script/Engine.CameraComponent|GetPostProcessSettings (Variables|Default|GetCamera)) _fstop _sensorwidth (Variables|/Script/Engine.SpringArmComponent|GetTargetArmLength (Variables|Default|GetSpringArm)))
  (CallFunction|UpdateCameraZoom))

(event EventHeal
  (params (HealAmount :type Float%20%28double-precision%29))
  ;[0.15 0.15 0.15 0.5] Stat Interface
  (Default|Heal (Variables|Default|GetStat%20Component) HealAmount))

(event EventDamage
  (params (DamageAmount :type Float%20%28double-precision%29))
  ;[0.15 0.15 0.15 0.5] Stat Interface
  (Default|Damage (Variables|Default|GetStat%20Component) DamageAmount))

(event EventSetMaxHP
  (params (MaxHP :type Float%20%28double-precision%29))
  ;[0.15 0.15 0.15 0.5] Stat Interface
  (Default|SetMaxHP (Variables|Default|GetStat%20Component) MaxHP))

(event EventIncreaseMaxHP
  (params (IncreaseAmount :type Float%20%28double-precision%29))
  ;[0.15 0.15 0.15 0.5] Stat Interface
  (Default|IncreaseMaxHP (Variables|Default|GetStat%20Component) IncreaseAmount))

(event EventDecreaseMaxHP
  (params (DeacreaseAmount :type Float%20%28double-precision%29))
  ;[0.15 0.15 0.15 0.5] Stat Interface
  (Default|DecreaseMaxHP (Variables|Default|GetStat%20Component) DeacreaseAmount))

(event EventSetStat
  (params (Stat :type F%20Player%20Stat%20Structure))
  ;[0.15 0.15 0.15 0.5] Stat Interface
  (Default|SetStat (Variables|Default|GetStat%20Component) Stat))

(event Input|MouseEvents|DebugKeyMouseWheelAxis
  (params (Key :type Key%20Structure :default "None") (ActionValue :type Input%20Action%20Value%20Structure))
  (bind _zoombounds (Variables|Zoom|GetZoomBounds))
  (:Pressed
    (if (and (!= (.x ActionValue) 0.0) (not (Audio|Components|Audio|IsPlaying (Variables|Default|GetZoom))))
      (Variables|Zoom|SetZoomMultiplier (Math|Float|Clamp(Float) (+ (Variables|Zoom|GetZoomMultiplier) (* (.x ActionValue) -1.0)) (.x _zoombounds) (.y _zoombounds))))))

(fn ConstructionScript
  (|CallParentFunction))

(fn UpdateCameraZoom
  (Variables|/Script/Engine.SpringArmComponent|SetTargetArmLength (Variables|Default|GetSpringArm) (Math|Interpolation|FInterpTo (Variables|/Script/Engine.SpringArmComponent|GetTargetArmLength (Variables|Default|GetSpringArm)) (* (Variables|Zoom|GetZoomMultiplier) (Variables|Zoom|GetZoomStep)) (Utilities|Time|GetWorldDeltaSeconds) 2.0)))

(fn ComputeFocalDistance
  (return (Math|Vector|Distance(Vector) (Transformation|GetActorLocation) (Transformation|GetWorldLocation (Variables|Default|GetCamera)))))

(fn SetPlayerSaveInformation
  (bind _savegame (Class|BPISaveGame|GetSelectedGameData(Message) (Game|GetGameInstance)))
  (bind _output_get (LocalVariables|SetSave _savegame))
  (Utilities|IsValid _output_get
    (:Is%20Valid
      (if (not (== (Utilities|Struct|BreakFPlayerSave (Variables|/Game/XXII/Core/SaveGame/BP_XXIISaveGame.BP_XXIISaveGame_C|GetPlayerSave (LocalVariables|GetSave))) (Math|Transform|MakeTransform "0, 0, 0")))
        (Transformation|SetActorTransform (Utilities|Struct|BreakFPlayerSave (Variables|/Game/XXII/Core/SaveGame/BP_XXIISaveGame.BP_XXIISaveGame_C|GetPlayerSave (LocalVariables|GetSave))))
        (if (not (CallFunction|IsStatDefault (Utilities|Struct|BreakFPlayerSave (Variables|/Game/XXII/Core/SaveGame/BP_XXIISaveGame.BP_XXIISaveGame_C|GetPlayerSave (LocalVariables|GetSave)))))
          (Variables|/Game/XXII/Core/Stat/BP_StatComponent.BP_StatComponent_C|SetStat (Variables|Default|GetStat%20Component) (Utilities|Struct|BreakFPlayerSave (Variables|/Game/XXII/Core/SaveGame/BP_XXIISaveGame.BP_XXIISaveGame_C|GetPlayerSave (LocalVariables|GetSave)))))))))

(fn GetStat
  (return (Variables|/Game/XXII/Core/Stat/BP_StatComponent.BP_StatComponent_C|GetStat (Variables|Default|GetStat%20Component))))