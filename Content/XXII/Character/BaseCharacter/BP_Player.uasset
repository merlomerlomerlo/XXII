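; Player character Blueprint that handles camera-relative movement, yaw look, dash, and slash and aimed-shot attacks delegated to CombatComponent.
; Most actions are gated by IsDoingNone, which checks combat, dash, fall and aim states.
; Mouse wheel sets a clamped zoom multiplier; Tick interpolates spring arm length and updates depth-of-field settings to match, leaving the Zoom timeline unused.
; BeginPlay restores transform and stats from the selected save.
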(event Input|EnhancedActionEvents|EnhancedInputActionIA_Move
  (params (ActionValue :type Vector%202D%20Structure) (ElapsedSeconds :type Float%20%28double-precision%29) (TriggeredSeconds :type Float%20%28double-precision%29) (InputAction :type Input%20Action%20Object%20Reference :default "/Game/Input/Actions/IA_Move.IA_Move"))
  (bind _camera (Variables|Default|GetCamera))
  (bind _returnvalue (Transformation|GetWorldRotation _camera))
  (:Triggered
    (Utilities|IsDoingNone true true true false false
      (:Output
        (Variables|Default|SetIsMoving true)
        (Pawn|Input|AddMovementInput (Math|Vector|GetForwardVector (Math|Rotator|MakeRotator (.roll _returnvalue) 0.0 (.yaw _returnvalue))) (.y (Input|EnhancedActionValues|GetIA_Move)) false)
        (Pawn|Input|AddMovementInput (Math|Vector|GetRightVector (Math|Rotator|MakeRotator 0.0 0.0 (.yaw (Transformation|GetWorldRotation (Variables|Default|GetCamera))))) (.x (Input|EnhancedActionValues|GetIA_Move)) false))))
  (:Canceled
    (Variables|Default|SetIsMoving false :!label _label))
  (:Completed
    (goto _label)))

(event Input|EnhancedActionEvents|EnhancedInputActionIA_Slash
  (params (ActionValue :type Boolean) (ElapsedSeconds :type Float%20%28double-precision%29) (TriggeredSeconds :type Float%20%28double-precision%29) (InputAction :type Input%20Action%20Object%20Reference :default "/Game/Input/Actions/IA_Slash.IA_Slash"))
  (:Started
    (Utilities|IsDoingNone false true true false true
      (:Output
        (Class|CombatComponent|QueueAttack (Variables|Default|GetCombatComponent)))))
  (:Completed
    (Class|CombatComponent|ReleaseAttack (Variables|Default|GetCombatComponent))))

(event Input|EnhancedActionEvents|EnhancedInputActionIA_MouseLook
  (params (ActionValue :type Vector%202D%20Structure) (ElapsedSeconds :type Float%20%28double-precision%29) (TriggeredSeconds :type Float%20%28double-precision%29) (InputAction :type Input%20Action%20Object%20Reference :default "/Game/Input/Actions/IA_MouseLook.IA_MouseLook"))
  (Pawn|Input|AddControllerYawInput (.x ActionValue)))

(event Input|EnhancedActionEvents|EnhancedInputActionIA_Dash
  (params (ActionValue :type Boolean) (ElapsedSeconds :type Float%20%28double-precision%29) (TriggeredSeconds :type Float%20%28double-precision%29) (InputAction :type Input%20Action%20Object%20Reference :default "/Game/Variant_Platforming/Input/Actions/IA_Dash.IA_Dash"))
  (Utilities|IsDoingNone true true true false true
    (:Output
      (Class|XXIICharacter|DoDash))))

(event Input|EnhancedActionEvents|EnhancedInputActionIA_Aim
  (params (ActionValue :type Boolean) (ElapsedSeconds :type Float%20%28double-precision%29) (TriggeredSeconds :type Float%20%28double-precision%29) (InputAction :type Input%20Action%20Object%20Reference :default "/Game/Input/Actions/IA_Aim.IA_Aim"))
  (bind _combatcomponent (Variables|Default|GetCombatComponent))
  (:Started
    (Class|CombatComponent|StartAiming _combatcomponent))
  (:Canceled
    (Class|CombatComponent|StopAiming _combatcomponent :!label _label))
  (:Completed
    (goto _label)))

(event Input|EnhancedActionEvents|EnhancedInputActionIA_Shoot
  (params (ActionValue :type Boolean) (ElapsedSeconds :type Float%20%28double-precision%29) (TriggeredSeconds :type Float%20%28double-precision%29) (InputAction :type Input%20Action%20Object%20Reference :default "/Game/Input/Actions/IA_Shoot.IA_Shoot"))
  (:Started
    (if (Variables|/Script/XXII.CombatComponent|GetIsAiming (Variables|Default|GetCombatComponent))
      (Class|CombatComponent|Shoot (Variables|Default|GetCombatComponent))
      (Utilities|FlowControl|Delay 0.4)
      (Class|CombatComponent|StopAiming (Variables|Default|GetCombatComponent)))))

(event EventBeginPlay
  (bind (_fstop _sensorwidth) (Utilities|GetZoomPPSettings))
  (|CallParentFunction)
  (Save|SetPlayerSaveInformation)
  (bind _output_get (Variables|/Script/Engine.SpringArmComponent|SetTargetArmLength (Variables|Default|GetSpringArm) (* (Variables|Zoom|GetZoomMultiplier) (Variables|Zoom|GetZoomStep))))
  (Utilities|Struct|SetmembersinPostProcessSettings (Variables|/Script/Engine.CameraComponent|GetPostProcessSettings (Variables|Default|GetCamera)) _fstop _sensorwidth _output_get))

(event EventTick
  (params (DeltaSeconds :type Float%20%28single-precision%29))
  (bind (_fstop _sensorwidth) (Utilities|GetZoomPPSettings))
  (Utilities|Struct|SetmembersinPostProcessSettings (Variables|/Script/Engine.CameraComponent|GetPostProcessSettings (Variables|Default|GetCamera)) _fstop _sensorwidth (Variables|/Script/Engine.SpringArmComponent|GetTargetArmLength (Variables|Default|GetSpringArm)))
  (Camera|UpdateCameraZoom))

(event EventOnMovementModeChanged
  (params (PrevMovementMode :type EMovementMode%20Enum :default "MOVE_None") (NewMovementMode :type EMovementMode%20Enum :default "MOVE_None") (PrevCustomMode :type Byte :default 0) (NewCustomMode :type Byte :default 0))
  (if (Utilities|Enum|Equal(Enum) NewMovementMode "MOVE_Falling")
    (Class|XXIICharacter|EndDash)))

(event Input|MouseEvents|DebugKeyMouseWheelAxis
  (params (Key :type Key%20Structure :default "None") (ActionValue :type Input%20Action%20Value%20Structure))
  (bind _zoombounds (Variables|Zoom|GetZoomBounds))
  (:Pressed
    (if (and (!= (.x ActionValue) 0.0) (not (Audio|Components|Audio|IsPlaying (Variables|Default|GetZoom))))
      (Variables|Zoom|SetZoomMultiplier (Math|Float|Clamp(Float) (+ (Variables|Zoom|GetZoomMultiplier) (* (.x ActionValue) -1.0)) (.x _zoombounds) (.y _zoombounds))))))

(fn ConstructionScript
  (|CallParentFunction))

(fn UpdateCameraZoom
  (Variables|/Script/Engine.SpringArmComponent|SetTargetArmLength (Variables|Default|GetSpringArm) (Math|Interpolation|FInterpTo (Variables|/Script/Engine.SpringArmComponent|GetTargetArmLength (Variables|Default|GetSpringArm)) (* (Variables|Zoom|GetZoomMultiplier) (Variables|Zoom|GetZoomStep)) (Utilities|Time|GetWorldDeltaSeconds) 2.0)))

(fn SetPlayerSaveInformation
  (bind _savegame (Class|BPISaveGame|GetSelectedGameData(Message) (Game|GetGameInstance)))
  (bind _output_get (LocalVariables|SetSave _savegame))
  (Utilities|IsValid _output_get
    (:Is%20Valid
      (if (not (== (Utilities|Struct|BreakFPlayerSave (Variables|/Game/XXII/Core/SaveGame/BP_XXIISaveGame.BP_XXIISaveGame_C|GetPlayerSave (LocalVariables|GetSave))) (Math|Transform|MakeTransform "0, 0, 0")))
        (Transformation|SetActorTransform (Utilities|Struct|BreakFPlayerSave (Variables|/Game/XXII/Core/SaveGame/BP_XXIISaveGame.BP_XXIISaveGame_C|GetPlayerSave (LocalVariables|GetSave))))
        (if (not (CallFunction|IsStatDefault (Utilities|Struct|BreakFPlayerSave (Variables|/Game/XXII/Core/SaveGame/BP_XXIISaveGame.BP_XXIISaveGame_C|GetPlayerSave (LocalVariables|GetSave)))))
          (Variables|/Game/XXII/Core/Stat/BP_StatComponent.BP_StatComponent_C|SetStat (Variables|Default|GetStat%20Component) (Utilities|Struct|BreakFPlayerSave (Variables|/Game/XXII/Core/SaveGame/BP_XXIISaveGame.BP_XXIISaveGame_C|GetPlayerSave (LocalVariables|GetSave)))))))))