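; BP_Boss_0 is a boss that always turns to face the player character and makes its entrance when the fight trigger is hit.
; The first BP_BaseCharacter overlap on FightTriggerCapsule plays a timeline that moves the boss from its starting position to a target actor's location.
; After a short pause it fires one volley of forward-facing projectiles, using a delayed loop macro around a single-shot spawn macro.
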(event OnActorBeginOverlap(FightTriggerCapsule)
  (params (OverlappedActor :type Actor%20Object%20Reference) (OtherActor :type Actor%20Object%20Reference))
  (Utilities|Casting|CastToBP_BaseCharacter OtherActor)
  (if (not (Variables|Default|GetSpawned))
    (Variables|Default|SetSpawned true)
    (bind _lerplocation (Timeline|Spawn Play)
      (:Update
        (Transformation|SetActorLocation (Math|Vector|Lerp(Vector) (Variables|Default|GetStartingLocation) (Variables|Default|GetSpawnLocation) _lerplocation) false false))
      (:Finished
        (Utilities|FlowControl|Delay 1.0)
        (Utilities|ShootXProjectiles 0.3 3)))))

(event EventBeginPlay
  (Variables|Default|SetSpawnLocation (Transformation|GetActorLocation (Variables|Default|GetSpawnLocationTarget)))
  (Variables|Default|SetStartingLocation (Transformation|GetActorLocation))
  (bind _returnvalue (Actor|GetActorOfClass "/Script/XXII.XXIICharacter"))
  (Variables|Default|SetCharacter _returnvalue))

(event Collision|EventActorBeginOverlap
  (params (OtherActor :type Actor%20Object%20Reference)))

(event EventTick
  (params (DeltaSeconds :type Float%20%28single-precision%29))
  (Transformation|SetActorRotation (Math|Rotator|FindLookatRotation (Transformation|GetActorLocation) (Transformation|GetActorLocation (Variables|Default|GetCharacter)))))

(fn ConstructionScript)