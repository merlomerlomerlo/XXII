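; BP_Dummy is an enemy character Blueprint with a melee attack and a ragdoll death.
; Its attack event sphere-traces between two mesh sockets and hits each actor once per attack, clearing the hit list when the attack ends.
; Hits send damage, and character victims are also launched along the dummy's forward vector with a Niagara effect and brief global slow-motion hit-stop.
; On death the mesh switches to physics simulation.
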(event Custom|TraceAttack_1
  (bind (_outhit _returnvalue) (Class|KismetSystemLibrary|SphereTraceSinglebyProfile (Transformation|GetSocketLocation (Variables|Character|GetMesh) (Variables|Enemy|Attack|Trace|GetBoneNameStartAttackTrace)) (Transformation|GetSocketLocation (Variables|Character|GetMesh) (Variables|Enemy|Attack|Trace|GetBoneNameEndAttackTrace)) 5.0 "Pawn" false 0 "ForDuration" true "(R=1.000000,G=0.000000,B=0.000000,A=1.000000)" "(R=0.000000,G=1.000000,B=0.000000,A=1.000000)" 1.0))
  (if _returnvalue
    (if (not (Utilities|Array|ContainsItem (Variables|Enemy|Attack|Trace|GetHittedActor) (.HitActor (Collision|BreakHitResult _outhit))))
      (Utilities|Array|AddUnique (Variables|Enemy|Attack|Trace|GetHittedActor) (.HitActor (Collision|BreakHitResult _outhit)))
      (Class|StatInterface|Damage(Message) (.HitActor (Collision|BreakHitResult _outhit)) 1.0)
      (bind _ascharacter (Utilities|Casting|CastToCharacter (.HitActor (Collision|BreakHitResult _outhit))))
      (Character|LaunchCharacter _ascharacter (* (Transformation|GetActorForwardVector) 2.5e+03) false false)
      (Niagara|SpawnSystematLocation "/Game/Variant_Combat/VFX/NS_Damage.NS_Damage" (.ImpactPoint (Collision|BreakHitResult _outhit)))
      (Utilities|Time|SetGlobalTimeDilation 0.1)
      (Utilities|FlowControl|Delay 0.05)
      (Utilities|Time|SetGlobalTimeDilation 1.0))))

(event EventEndAttack
  (Utilities|Array|Clear (Variables|Enemy|Attack|Trace|GetHittedActor))
  (|CallParentFunction))

(fn ConstructionScript
  (|CallParentFunction))

(fn OnEnemyDeath
  (|CallParentFunction)
  (Physics|SetSimulatePhysics (Variables|Character|GetMesh) true)
  (Collision|SetCollisionEnabled (Variables|Character|GetMesh) "PhysicsOnly"))