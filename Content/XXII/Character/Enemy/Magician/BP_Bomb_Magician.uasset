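; Bomb projectile of the Magician enemy that explodes and leaves a visible damage area that hurts the player.
; On hit it hides the bomb, plays explosion effect, sound and camera shake, then moves and enables the damage area and sets a lifespan for cleanup.
; Player overlap with that area sends a damage message, and the construction script sizes its collision from the area's scale.
; Tick keeps a shadow under the bomb at a set height.
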(event OnComponentBeginOverlap(DamageAreaCollision)
  (params (OverlappedComponent :type Primitive%20Component%20Object%20Reference) (OtherActor :type Actor%20Object%20Reference) (OtherComp :type Primitive%20Component%20Object%20Reference) (OtherBodyIndex :type Integer) (bFromSweep :type Boolean) (SweepResult :type Hit%20Result%20Structure%20%28by%20ref%29))
  (if (== OtherActor (Game|Player|GetPlayerPawn 0))
    (Class|StatInterface|Damage(Message) (Game|Player|GetPlayerPawn 0) 1.0)))

(event OnComponentBeginOverlap(SphereTrigger)
  (params (OverlappedComponent :type Primitive%20Component%20Object%20Reference) (OtherActor :type Actor%20Object%20Reference) (OtherComp :type Primitive%20Component%20Object%20Reference) (OtherBodyIndex :type Integer) (bFromSweep :type Boolean) (SweepResult :type Hit%20Result%20Structure%20%28by%20ref%29))
  (Utilities|IsValid OtherActor
    (:Is%20Valid
      (Collision|SetCollisionEnabled (Variables|Default|GetSphereTrigger) "NoCollision"))))

(event Custom|OnHitSomething
  (bind _spherecollision (Variables|Default|GetSphereCollision))
  (bind _returnvalue (Transformation|GetWorldLocation _spherecollision))
  (Rendering|SetVisibility (Variables|Default|GetBomb) false true)
  (Rendering|SetVisibility (Variables|Default|GetSphereCollision) false true)
  (Niagara|SpawnSystematLocation "/Niagara/DefaultAssets/Templates/Systems/SimpleExplosion.SimpleExplosion" (Transformation|GetWorldLocation (Variables|Default|GetSphere)))
  (CameraShakes|StartCameraShake (Game|GetPlayerCameraManager 0) "/Game/Variant_Combat/Blueprints/BP_CameraShake_Hit_Enemy.BP_CameraShake_Hit_Enemy_C" 1.0 "CameraLocal" "0, 0, 0")
  (Audio|PlaySoundatLocation "/Engine/VREditor/Sounds/VR_ungrab.VR_ungrab" (Transformation|GetWorldLocation (Variables|Default|GetSphere)) "0, 0, 0" 0.5 1.0 0.0 0 0 0 0)
  (Rendering|SetVisibility (Variables|Default|GetArea) true false)
  (Collision|SetCollisionEnabled (Variables|Default|GetDamageAreaCollision) "QueryOnly")
  (Transformation|SetWorldLocation (Variables|Default|GetDamageArea) (Math|Vector|MakeVector (.x _returnvalue) (.y _returnvalue) (.z _returnvalue)) false false)
  (Actor|SetLifeSpan 0.0)
  (Actor|SetLifeSpan 1e+01))

(event EventBeginPlay
  (Utilities|Time|SetTimerbyEvent (EventDispatchers|CreateEvent :!event Custom|OnHitSomething) 0.1 false true 2.0))

(event EventTick
  (params (DeltaSeconds :type Float%20%28single-precision%29))
  (bind _sphere (Variables|Default|GetSphere))
  (bind _returnvalue (Transformation|GetWorldLocation _sphere))
  (Transformation|SetWorldLocation (Variables|Default|GetSphereShadow) (Math|Vector|MakeVector (.x _returnvalue) (.y _returnvalue) (Variables|Default|GetShadowWorldZPosition)) false false))

(fn ConstructionScript
  (Components|Sphere|SetSphereRadius (Variables|Default|GetDamageAreaCollision) (* 5e+01 (.x (Variables|/Script/Engine.SceneComponent|GetRelativeScale3D (Variables|Default|GetArea)))) true))