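; BP_Magician is an enemy that patrols an arena path while firing orbs.
; On BeginPlay it takes the spline from the path actor and starts a looping timer that spawns BP_Orb projectiles with its configured speed and damage.
; Each Tick it moves along the spline at a fixed height, reversing at either end, and rotates to face FacingTarget.
; The orb spawn offset scales only the Y component of the forward vector.
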(event Custom|ShootOrb
  (Game|SpawnActorfromClass "/Game/XXII/Character/Enemy/Magician/BP_Orb.BP_Orb_C" (Math|Transform|MakeTransform (+ (* (Transformation|GetActorForwardVector) "0.000000,100.000000,0.000000") (Transformation|GetActorLocation)) (Transformation|GetActorRotation) "1.000000,1.000000,1.000000") "AlwaysSpawn" "MultiplyWithRoot" 0 (Variables|Orbs|GetOrbSpeed) (Variables|Orbs|GetOrbDamage) 0))

(event EventBeginPlay
  (Utilities|Time|SetTimerbyEvent (delegate Custom|ShootOrb) (Variables|Orbs|GetOrbSpawnRate) true)
  (bind _output_get (Variables|Default|SetArenaPath (Actor|GetComponentbyClass (Variables|Movement|GetArenaPathActor) "/Script/Engine.SplineComponent")))
  (Variables|Movement|SetArenaPathLength (Spline|GetSplineLength _output_get))
  (if (Variables|Movement|GetIsMovingClockwise)
    (Variables|Movement|SetCurrentDistance 0.0)
    (else
      (Variables|Movement|SetCurrentDistance (Variables|Movement|GetArenaPathLength)))))

(event EventTick
  (params (DeltaSeconds :type Float%20%28single-precision%29))
  (bind _movementspeed (Variables|Movement|GetMovementSpeed))
  (bind _returnvalue (* DeltaSeconds _movementspeed))
  (if (Variables|Movement|GetIsMovingClockwise)
    (Variables|Movement|SetNewDistance (+ (Variables|Movement|GetCurrentDistance) _returnvalue))
    (if (> (Variables|Movement|GetNewDistance) (Variables|Movement|GetArenaPathLength))
      (Variables|Movement|SetNewDistance (Variables|Movement|GetArenaPathLength))
      (Variables|Movement|SetIsMovingClockwise false))
    (else
      (Variables|Movement|SetNewDistance (- (Variables|Movement|GetCurrentDistance) _returnvalue))
      (if (<= (Variables|Movement|GetNewDistance) 0.0)
        (Variables|Movement|SetNewDistance 0.0)
        (Variables|Movement|SetIsMovingClockwise true))))
  (Variables|Movement|SetCurrentDistance (Variables|Movement|GetNewDistance))
  (Transformation|SetActorLocation (Math|Vector|MakeVector (.x (Spline|GetLocationatDistanceAlongSpline (Variables|Default|GetArenaPath) (Variables|Movement|GetCurrentDistance) "World")) (.y (Spline|GetLocationatDistanceAlongSpline (Variables|Default|GetArenaPath) (Variables|Movement|GetCurrentDistance) "World")) 1.1e+02) false false)
  (Transformation|SetActorRotation (Math|Rotator|FindLookatRotation (Transformation|GetActorLocation) (Variables|Movement|GetFacingTarget))))

(fn ConstructionScript
  (|CallParentFunction))