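; Magician boss enemy that circles by rotating its actor around an offset mesh and enables attacks through an AI blackboard flag.
; Timers fire orbs at the player, bomb volleys use suggested arc velocities, and both signal when finished.
; The laser attack reuses one timeline with swapped finish callbacks to rise, slam down with shockwaves, sweep four rotating lasers, then return to circling.
; RandomAttack only prints its pick.
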(event Custom|BombAttack
  (Utilities|FlowControl|Delay 5.0)
  (bind _returnvalue (Math|Random|RandomIntegerinRange 0 (Variables|Character|01-Actions|GetMaxBombAmount) :!label _label))
  (Development|PrintText (Utilities|Text|FormatText "Bomb attack: {boattk} -> Amount: {boam}" (+ (Variables|Character|01-Actions|GetCurrentBombAttack) 1) _returnvalue))
  (Character|01-Actions|BombAttackFunction :!label _label_2)
  (bind _result (Math|Integer|IncrementInt (Variables|Character|01-Actions|GetCurrentBombAmount))
    (:%20%20
      (if (< _result _returnvalue)
        (Utilities|FlowControl|Delay 1.5)
        (goto _label_2)
        (else
          (Variables|Character|01-Actions|SetCurrentBombAmount 0)
          (bind _result_2 (Math|Integer|IncrementInt (Variables|Character|01-Actions|GetCurrentBombAttack))
            (:%20%20
              (if (< _result_2 (Variables|Character|01-Actions|GetMaxBombAttack))
                (Utilities|FlowControl|Delay 5.0)
                (goto _label)
                (else
                  (Variables|Character|01-Actions|SetMaxBombAttack 0)
                  (Utilities|FlowControl|Delay 0.2)
                  (Default|CallOnFinishAttack))))))))))

(event Custom|OnBombExplosion
  (params (DestroyedActor :type Actor%20Object%20Reference)))

(event Custom|LaserShockWaveAttack
  (Collision|SetCollisionEnabled (Variables|Default|GetLaser2) "QueryOnly")
  (Variables|Character|99-Utility|SetDefaultActorPosition (Transformation|GetActorLocation))
  (CallFunction|ChangePosition))

(event Custom|Random%20Attack
  (bind _returnvalue (Math|Random|RandomIntegerinRange 0 2))
  (Development|PrintString (Utilities|Select :Index _returnvalue :Option%200 "Orb" :Option%201 "Bomb" :Option%202 "Laser"))
  (switch int _returnvalue))

(event Custom|ChangePosition
  (Class|TimelineComponent|SetTimelineFinishedFunc (Variables|Default|GetMoveToUp) (EventDispatchers|CreateEvent :!event Custom|ShockLaserPositionPH1))
  (Components|Timeline|SetNewTime (Variables|Default|GetMoveToUp) 1.0)
  (bind _alpha (Timeline|MoveToUp Play)
    (:Update
      (Transformation|SetActorLocation (Math|Vector|Lerp(Vector) (Variables|Character|99-Utility|GetDefaultActorPosition) (+ (Variables|Character|99-Utility|GetDefaultActorPosition) "0.000000,0.000000,1000.000000") _alpha) false false))))

(event Custom|OnLasersBeginOverlap
  (params (OverlappedComponent :type Primitive%20Component%20Object%20Reference) (OtherActor :type Actor%20Object%20Reference) (OtherComp :type Primitive%20Component%20Object%20Reference) (OtherBodyIndex :type Integer) (bFromSweep :type Boolean) (SweepResult :type Hit%20Result%20Structure%20%28by%20ref%29))
  (if (== OtherActor (Game|Player|GetPlayerPawn 0))
    (Class|StatInterface|Damage(Message) (Game|Player|GetPlayerPawn 0) 1.0)))

(event Custom|ShockLaserPositionPH1
  (if (> (Components|Timeline|GetPlaybackPosition (Variables|Default|GetMoveToUp)) 0.0)
    (Transformation|SetRelativeLocation (Variables|Character|GetMesh) "0, 0, 0" false false)
    (Variables|Default|SetbCanBossStart false)
    (Variables|Character|99-Utility|SetbMoveLaser true)
    (Transformation|SetActorRotation "0.000000,-90.000000,0.000000")
    (Components|Timeline|SetNewTime (Variables|Default|GetMoveToUp) 0.25)
    (Components|Timeline|ReversefromEnd (Variables|Default|GetMoveToUp))
    (else
      (Audio|PlaySound2D "/Engine/VREditor/Sounds/VR_ungrab.VR_ungrab" 1.0 1.0 0.0 0 0)
      (CameraShakes|StartCameraShake (Game|GetPlayerCameraManager 0) "/Game/Variant_Combat/Blueprints/BP_CameraShake_Hit_Enemy.BP_CameraShake_Hit_Enemy_C" 1.0 "CameraLocal" "0, 0, 0")
      (Game|SpawnActorfromClass "/Game/XXII/Character/Enemy/Magician/BP_ShockWave_Magician.BP_ShockWave_Magician_C" (Math|Transform|MakeTransform (.location (Transformation|GetActorTransform)) "0, 0, 0" "1.000000,1.000000,1.000000") "Undefined" "MultiplyWithRoot" 0 0)
      (Utilities|FlowControl|Delay 0.2)
      (Game|SpawnActorfromClass "/Game/XXII/Character/Enemy/Magician/BP_ShockWave_Magician.BP_ShockWave_Magician_C" (Math|Transform|MakeTransform (.location (Transformation|GetActorTransform)) "0, 0, 0" "1.000000,1.000000,1.000000") "Undefined" "MultiplyWithRoot" 0 0)
      (Utilities|FlowControl|Delay 3.0)
      (Development|SetHiddeninGame (Variables|Default|GetLaser2) false false)
      (Audio|PlaySound2D "/Engine/VREditor/Sounds/UI/Laser_Push.Laser_Push" 1.0 1.0 0.0 0 0)
      (Utilities|FlowControl|Delay 1.0)
      (|LaserPhase
        (:ExtendedLaser
          (Variables|Default|SetbCanBossStart true))
        (:EndPhase
          (Class|TimelineComponent|SetTimelineFinishedFunc (Variables|Default|GetMoveToUp) (EventDispatchers|CreateEvent :!event Custom|ShockLaserPositionPH2))
          (Components|Timeline|SetNewTime (Variables|Default|GetMoveToUp) 1.0)
          (Components|Timeline|PlayfromStart (Variables|Default|GetMoveToUp)))))))

(event Custom|ShockLaserPositionPH2
  (if (> (Components|Timeline|GetPlaybackPosition (Variables|Default|GetMoveToUp)) 0.0)
    (Transformation|SetRelativeLocation (Variables|Character|GetMesh) (Variables|Character|99-Utility|GetDefaultRelativeMeshPosition) false false)
    (Variables|Default|SetbCanBossStart false)
    (Variables|Character|99-Utility|SetbMoveLaser false)
    (Transformation|SetRelativeRotation (Variables|Default|GetLasers) "0, 0, 0" false false)
    (Components|Timeline|SetNewTime (Variables|Default|GetMoveToUp) 0.25)
    (Components|Timeline|ReversefromEnd (Variables|Default|GetMoveToUp))
    (else
      (Variables|Default|SetbCanBossStart true)
      (CallFunction|RandomAttack))))

(event Custom|OrbAttackTimer
  (bind _output_get (Variables|Character|01-Actions|SetOrbAttackCurrentDuration (+ (Variables|Character|01-Actions|GetOrbAttackCurrentDuration) 0.1)))
  (if (>= _output_get (Variables|Character|01-Actions|GetOrbAttackDuration))
    (Utilities|Time|ClearandInvalidateTimerbyHandle (Variables|Character|99-Utility|GetOrbAttackHandler))
    (Utilities|Time|ClearandInvalidateTimerbyHandle (Variables|Character|99-Utility|GetOrbAttackTimerHandler))
    (Utilities|FlowControl|Delay 5.0)
    (Default|CallOnFinishAttack)))

(event EventBeginPlay
  (|CallParentFunction)
  (Variables|Character|99-Utility|SetDefaultRelativeMeshPosition (Variables|/Script/Engine.SceneComponent|GetRelativeLocation (Variables|Character|GetMesh)))
  (Collision|BindEventtoOnComponentBeginOverlap (Variables|Default|GetLaser0) (EventDispatchers|CreateEvent :!event Custom|OnLasersBeginOverlap)))

(event EventStartBoss
  (|CallParentFunction)
  (Utilities|FlowControl|Delay 2.0)
  (CallFunction|TurnonAttacking))

(event EventTick
  (params (DeltaSeconds :type Float%20%28single-precision%29))
  (if (Variables|Default|GetbCanBossStart)
    (Character|01-Actions|Move)))

(event EventDestroyed
  (|CallParentFunction)
  (Niagara|SpawnSystematLocation "/Niagara/DefaultAssets/Templates/Systems/SimpleExplosion.SimpleExplosion" (Transformation|GetWorldLocation (Variables|Character|GetMesh)))
  (Audio|PlaySound2D "/Engine/VREditor/Sounds/VR_teleport.VR_teleport" 1.0 1.0 0.0 0 0))

(fn ConstructionScript
  (|CallParentFunction))

(fn Move
  (if (not (Variables|Character|99-Utility|GetbMoveLaser))
    (|BossMovement)
    (else
      (|LaserRotation))))

(fn OrbAttack
  (Variables|Character|01-Actions|SetOrbAttackCurrentDuration 0.0)
  (bind _returnvalue (Utilities|Time|SetTimerbyEvent (EventDispatchers|CreateEvent :!event OrbAttackFunction) (Variables|Character|01-Actions|GetOrbFireRate) true true))
  (Variables|Character|99-Utility|SetOrbAttackHandler _returnvalue)
  (bind _returnvalue_2 (Utilities|Time|SetTimerbyEvent (EventDispatchers|CreateEvent :!event Custom|OrbAttackTimer) 0.1 true false 3.0))
  (Variables|Character|99-Utility|SetOrbAttackTimerHandler _returnvalue_2))

(fn OrbAttackFunction
  (bind _returnvalue (Game|Player|GetPlayerPawn 0))
  (bind _mesh (Variables|Character|GetMesh))
  (bind _returnvalue_2 (Transformation|GetWorldTransform _mesh))
  (bind (_location _rotation _scale) (Math|Transform|BreakTransform _returnvalue_2))
  (bind _returnvalue_3 (+ _location "0.000000,50.000000,0.000000"))
  (bind _returnvalue_4 (Game|SpawnActorfromClass "/Game/XXII/Character/Enemy/Magician/BP_Orb_Magician.BP_Orb_Magician_C" (Math|Transform|MakeTransform _returnvalue_3 (Math|Rotator|FindLookatRotation _returnvalue_3 (+ (Transformation|GetActorLocation _returnvalue) (* (Transformation|GetActorForwardVector _returnvalue) 5e+01))) _scale) "Undefined" "MultiplyWithRoot" 0 (Variables|Character|01-Actions|GetOrbSpeed) 1.0 1e+01 0))
  (Utilities|IsValid _returnvalue_4
    (:Is%20Valid
      (Collision|IgnoreActorwhenMoving (Variables|/Game/XXII/Character/Enemy/Magician/BP_Orb_Magician.BP_Orb_Magician_C|GetSphereCollision _returnvalue_4) self true))))

(fn BombAttackFunction
  (bind _returnvalue (Game|Player|GetPlayerPawn 0))
  (bind _mesh (Variables|Character|GetMesh))
  (bind _returnvalue_2 (Transformation|GetActorLocation _returnvalue))
  (bind _returnvalue_3 (Transformation|GetWorldLocation _mesh))
  (bind _returnvalue_4 (Game|SpawnActorfromClass "/Game/XXII/Character/Enemy/Magician/BP_Bomb_Magician.BP_Bomb_Magician_C" (Math|Transform|MakeTransform (+ (.Location (Math|Transform|BreakTransform (Transformation|GetWorldTransform (Variables|Character|GetMesh)))) "0.000000,0.000000,150.000000") "0, 0, 0" "1.000000,1.000000,1.000000") "Undefined" "MultiplyWithRoot" 0 0))
  (bind _output_get (LocalVariables|SetNewBomb _returnvalue_4))
  (Game|BindEventtoOnDestroyed _output_get (EventDispatchers|CreateEvent :!event Custom|OnBombExplosion))
  (Utilities|FlowControl|Sequence
    (:then_0
      (bind (_outhit _returnvalue_5) (Collision|LineTraceByChannel _returnvalue_3 (+ _returnvalue_3 (* (Math|Vector|GetUpVector _mesh) -5e+01)) "TraceTypeQuery1" false 0 "Persistent"))
      (if _returnvalue_5
        (bind _newbomb (LocalVariables|GetNewBomb)
          (:then
            (Variables|/Game/XXII/Character/Enemy/Magician/BP_Bomb_Magician.BP_Bomb_Magician_C|SetShadowWorldZPosition _newbomb (.z (Transformation|GetActorLocation (.HitActor (Collision|BreakHitResult _outhit))))))
          (:else))))
    (:then_1
      (bind _outlaunchvelocity (Game|SuggestProjectileVelocityCustomArc (Transformation|GetActorLocation (LocalVariables|GetNewBomb)) (select (Math|Random|RandomBool) _returnvalue_2 (+ (* (Transformation|GetActorRightVector _returnvalue) (select (Math|Random|RandomBool) 1.5e+02 -1.5e+02)) _returnvalue_2)) 0.0 0.5))
      (Physics|SetPhysicsLinearVelocity (Variables|/Game/XXII/Character/Enemy/Magician/BP_Bomb_Magician.BP_Bomb_Magician_C|GetSphereCollision (LocalVariables|GetNewBomb)) _outlaunchvelocity false "None"))))

(fn TurnonAttacking
  (AI|Components|Blackboard|SetValueasBool (AI|GetBlackboard (AI|GetAIController self)) (Utilities|Name|MakeLiteralName "ShouldAttack") true))