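; BP_Orb_Magician is a projectile orb for the Magician enemy that damages the player on contact.
; On BeginPlay, its ProjectileMovement launches it along its local X axis at Speed, and a timer destroys it after LifespanSeconds.
; When SphereCollision begins overlapping the player pawn, it sends that pawn a DamageMessage with Damage and destroys itself, ignoring all other actors.
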(event OnComponentBeginOverlap(SphereCollision)
  (params (OverlappedComponent :type Primitive%20Component%20Object%20Reference) (OtherActor :type Actor%20Object%20Reference) (OtherComp :type Primitive%20Component%20Object%20Reference) (OtherBodyIndex :type Integer) (bFromSweep :type Boolean) (SweepResult :type Hit%20Result%20Structure%20%28by%20ref%29))
  (if (== OtherActor (Game|Player|GetPlayerPawn 0))
    (Class|StatInterface|Damage(Message) (Game|Player|GetPlayerPawn 0) (Variables|Default|GetDamage))
    (Actor|DestroyActor)))

(event Custom|Die
  (Actor|DestroyActor))

(event EventBeginPlay
  (Game|Components|ProjectileMovement|SetVelocityinLocalSpace (Variables|Default|GetProjectileMovement) (Math|Vector|MakeVector (Variables|Default|GetSpeed) 0.0 0.0))
  (Utilities|Time|SetTimerbyEvent (delegate Custom|Die) (Variables|Default|GetLifespanSeconds)))

(event Collision|EventActorBeginOverlap
  (params (OtherActor :type Actor%20Object%20Reference)))

(fn ConstructionScript)