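; Shockwave actor for the Magician enemy that expands outward and damages the player on contact.
; Tick adds a fixed step to the actor's scale on all axes every frame, so growth speed depends on frame rate.
; StaticWave's begin-overlap sends DamageMessage to player pawn 0 when that pawn is the overlapping actor.
; The graph never destroys the wave, and its node to disable StaticWave collision is unconnected.
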(event OnComponentBeginOverlap(StaticWave)
  (params (OverlappedComponent :type Primitive%20Component%20Object%20Reference) (OtherActor :type Actor%20Object%20Reference) (OtherComp :type Primitive%20Component%20Object%20Reference) (OtherBodyIndex :type Integer) (bFromSweep :type Boolean) (SweepResult :type Hit%20Result%20Structure%20%28by%20ref%29))
  (if (== OtherActor (Game|Player|GetPlayerPawn 0))
    (Class|StatInterface|Damage(Message) (Game|Player|GetPlayerPawn 0) 1.0)))

(event EventTick
  (params (DeltaSeconds :type Float%20%28single-precision%29))
  (Transformation|SetActorScale3D (+ (Transformation|GetActorScale3D) "0.100000,0.100000,0.100000")))

(fn ConstructionScript)