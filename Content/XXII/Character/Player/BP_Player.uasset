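; Player character that handles input for camera-relative movement, zoom, sprint, dash, chargeable slash, and aimed shooting.
; An IsDoingNone macro gates conflicting actions, while StatComponent supplies stamina checks and costs, and CombatComponent runs attacks and aiming.
; Held slashes scale Attack by stamina charged, and shooting also damages the player's own StatComponent.
; BeginPlay restores saved transform and stats; Tick interpolates spring-arm zoom and matches depth-of-field settings to it.
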(event OnChargedAttack(StatComponent)
  (params (StaminaChargeAmount :type Float%20%28double-precision%29))
  (Utilities|FlowControl|Sequence
    (:then_0
      (Utilities|FlowControl|Gate true) ; enters at Close
    )
    (:then_1
      (Utilities|Struct|SetmembersinObjectStat (Variables|/Game/XXII/Core/Stat/BP_StatComponent.BP_StatComponent_C|GetStat (Variables|Default|GetStat%20Component)) (Math|Float|Lerp 1.0 2.5 (/ StaminaChargeAmount (Variables|Combat|GetMaxStaminaChargeAttack))))
      (Class|CombatComponent|ReleaseAttack (Variables|Default|GetCombatComponent)))))

(event Custom|SprintDrainStamina
  (bind _result (Default|TryConsumeStamina (Variables|Default|GetStat%20Component) 0.25))
  (if (not _result)
    (Utilities|Time|ClearandInvalidateTimerbyHandle (stale Input|EnhancedActionEvents|EnhancedInputActionIA_Sprint _returnvalue))
    (Utilities|FlowControl|Gate false) ; enters at Open
  ))

(event Input|EnhancedActionEvents|EnhancedInputActionIA_Move
  (params (ActionValue :type Vector%202D%20Structure) (ElapsedSeconds :type Float%20%28double-precision%29) (TriggeredSeconds :type Float%20%28double-precision%29) (InputAction :type Input%20Action%20Object%20Reference :default "/Game/Input/Actions/IA_Move.IA_Move"))
  (bind _camera (Variables|Default|GetCamera))
  (bind _returnvalue (Transformation|GetWorldRotation _camera))
  (:Triggered
    (Utilities|IsDoingNone true true true false false
      (:Output
        (Variables|Default|SetIsMoving true)
        (Pawn|Input|AddMovementInput (Math|Vector|GetForwardVector (Math|Rotator|MakeRotator (.roll _returnvalue) 0.0 (.yaw _returnvalue))) (.y (Input|EnhancedActionValues|GetIA_Move)) false)
        (Pawn|Input|AddMovementInput (Math|Vector|GetRightVector (Math|Rotator|MakeRotator 0.0 0.0 (.yaw (Transformation|GetWorldRotation (Variables|Default|GetCamera))))) (.x (Input|EnhancedActionValues|GetIA_Move)) false))))
  (:Canceled
    (Variables|Default|SetIsMoving false :!label _label))
  (:Completed
    (goto _label)))

(event Input|EnhancedActionEvents|EnhancedInputActionIA_Slash
  (params (ActionValue :type Boolean) (ElapsedSeconds :type Float%20%28double-precision%29) (TriggeredSeconds :type Float%20%28double-precision%29) (InputAction :type Input%20Action%20Object%20Reference :default "/Game/Input/Actions/IA_Slash.IA_Slash"))
  (:Started
    (Utilities|IsDoingNone false true true false true
      (:Output
        (Utilities|FlowControl|Sequence
          (:then_0
            (goto _label Open))
          (:then_1
            (Class|CombatComponent|QueueAttack (Variables|Default|GetCombatComponent))
            (if (Default|CanDoAction (Variables|Default|GetStat%20Component) 0.5)
              (Default|StartChargeConsumeStamina (Variables|Default|GetStat%20Component) 0.5 0.5 (Variables|Combat|GetMaxStaminaChargeAttack))))))))
  (:Completed
    (Utilities|FlowControl|Gate true :!label _label
      (:Exit
        (Class|CombatComponent|ReleaseAttack (Variables|Default|GetCombatComponent))
        (Default|EndChargeConsumeStamina (Variables|Default|GetStat%20Component))))))

(event Input|EnhancedActionEvents|EnhancedInputActionIA_MouseLook
  (params (ActionValue :type Vector%202D%20Structure) (ElapsedSeconds :type Float%20%28double-precision%29) (TriggeredSeconds :type Float%20%28double-precision%29) (InputAction :type Input%20Action%20Object%20Reference :default "/Game/Input/Actions/IA_MouseLook.IA_MouseLook"))
  (Pawn|Input|AddControllerYawInput (.x ActionValue)))

(event Input|EnhancedActionEvents|EnhancedInputActionIA_Dash
  (params (ActionValue :type Boolean) (ElapsedSeconds :type Float%20%28double-precision%29) (TriggeredSeconds :type Float%20%28double-precision%29) (InputAction :type Input%20Action%20Object%20Reference :default "/Game/Variant_Platforming/Input/Actions/IA_Dash.IA_Dash"))
  (bind _fx_loc (Variables|Default|GetFX_Loc))
  (:Triggered
    (Utilities|IsDoingNone true true true false true
      (:Output
        (if (Default|CanDoAction (Variables|Default|GetStat%20Component) 1e+01)
          (Class|XXIICharacter|DoDash)
          (bind _returnvalue (Niagara|SpawnSystemAttached "/Game/XXII/VFX/Trails/VFX_DashTrail.VFX_DashTrail" _fx_loc "None" (Transformation|GetWorldLocation _fx_loc) (Math|Rotator|MakeRotator 0.0 0.0 (.yaw (Math|Rotator|MakeRotfromX (Transformation|GetActorForwardVector)))) "KeepWorldPosition" true))
          (Variables|Default|SetDash%20FX _returnvalue)))))
  (:Started
    (Utilities|IsDoingNone true true true false true
      (:Output
        (Utilities|FlowControl|Delay 0.5)
        (Animation|Montage|MontageStop (Components|SkeletalMesh|GetAnimInstance (Variables|Character|GetMesh)) 0.3 "/Game/XXII/Character/Player/Animations/Montages/DashMontage.DashMontage")))))

(event Input|EnhancedActionEvents|EnhancedInputActionIA_Aim
  (params (ActionValue :type Boolean) (ElapsedSeconds :type Float%20%28double-precision%29) (TriggeredSeconds :type Float%20%28double-precision%29) (InputAction :type Input%20Action%20Object%20Reference :default "/Game/Input/Actions/IA_Aim.IA_Aim"))
  (bind _combatcomponent (Variables|Default|GetCombatComponent))
  (:Started
    (Class|CombatComponent|StartAiming _combatcomponent)
    (Variables|/Game/XXII/Core/Stat/BP_StatComponent.BP_StatComponent_C|SetbIsAiming (Variables|Default|GetStat%20Component) true))
  (:Canceled
    (Class|CombatComponent|StopAiming _combatcomponent :!label _label)
    (Variables|/Game/XXII/Core/Stat/BP_StatComponent.BP_StatComponent_C|SetbIsAiming (Variables|Default|GetStat%20Component) false))
  (:Completed
    (goto _label)))

(event Input|EnhancedActionEvents|EnhancedInputActionIA_Shoot
  (params (ActionValue :type Boolean) (ElapsedSeconds :type Float%20%28double-precision%29) (TriggeredSeconds :type Float%20%28double-precision%29) (InputAction :type Input%20Action%20Object%20Reference :default "/Game/Input/Actions/IA_Shoot.IA_Shoot"))
  (:Started
    (if (Variables|/Script/XXII.CombatComponent|GetIsAiming (Variables|Default|GetCombatComponent))
      (bind _result (Default|TryConsumeStamina (Variables|Default|GetStat%20Component) 1e+01))
      (if _result
        (Class|CombatComponent|Shoot (Variables|Default|GetCombatComponent))
        (Default|Damage (Variables|Default|GetStat%20Component) 1.0)
        (Utilities|FlowControl|Delay 0.4)
        (Class|CombatComponent|StopAiming (Variables|Default|GetCombatComponent))))))

(event Input|EnhancedActionEvents|EnhancedInputActionIA_Sprint
  (params (ActionValue :type Boolean) (ElapsedSeconds :type Float%20%28double-precision%29) (TriggeredSeconds :type Float%20%28double-precision%29) (InputAction :type Input%20Action%20Object%20Reference :default "/Game/XXII/Core/Input/IA_Sprint.IA_Sprint"))
  (:Triggered
    (Utilities|IsDoingNone true true true false true
      (:Output
        (if (Default|CanDoAction (Variables|Default|GetStat%20Component) 0.5)
          (Variables|/Script/Engine.CharacterMovementComponent|SetMaxWalkSpeed (Variables|Character|GetCharacterMovement) 7.5e+02)
          (Utilities|FlowControl|Gate false :!label _label
            (:Exit
              (Utilities|FlowControl|Sequence
                (:then_0
                  (goto _label Close))
                (:then_1
                  (bind _returnvalue (Utilities|Time|SetTimerbyEvent (delegate Custom|SprintDrainStamina) 0.1 true true))))))
          (else
            (Variables|/Script/Engine.CharacterMovementComponent|SetMaxWalkSpeed (Variables|Character|GetCharacterMovement) 5e+02))))))
  (:Canceled
    (Variables|/Script/Engine.CharacterMovementComponent|SetMaxWalkSpeed (Variables|Character|GetCharacterMovement) 5e+02 :!label _label_2)
    (Utilities|Time|ClearandInvalidateTimerbyHandle _returnvalue)
    (goto _label Open))
  (:Completed
    (goto _label_2)))

(event EventBeginPlay
  (bind (_fstop _sensorwidth) (Utilities|GetZoomPPSettings))
  (|CallParentFunction)
  (Save|SetPlayerSaveInformation)
  (bind _output_get (Variables|/Script/Engine.SpringArmComponent|SetTargetArmLength (Variables|Default|GetSpringArm) (* (Variables|Zoom|GetZoomMultiplier) (Variables|Zoom|GetZoomStep))))
  (Utilities|Struct|SetmembersinPostProcessSettings (Variables|/Script/Engine.CameraComponent|GetPostProcessSettings (Variables|Default|GetCamera)) _fstop _sensorwidth _output_get))

(event EventTick
  (params (DeltaSeconds :type Float%20%28single-precision%29))
  (bind (_fstop _sensorwidth) (Utilities|GetZoomPPSettings))
  (Utilities|Struct|SetmembersinPostProcessSettings (Variables|/Script/Engine.CameraComponent|GetPostProcessSettings (Variables|Default|GetCamera)) _fstop _sensorwidth (Variables|/Script/Engine.SpringArmComponent|GetTargetArmLength (Variables|Default|GetSpringArm)))
  (Camera|UpdateCameraZoom))

(event EventTraceHitbox)

(event EventOnMovementModeChanged
  (params (PrevMovementMode :type EMovementMode%20Enum :default "MOVE_None") (NewMovementMode :type EMovementMode%20Enum :default "MOVE_None") (PrevCustomMode :type Byte :default 0) (NewCustomMode :type Byte :default 0))
  (if (Utilities|Enum|Equal(Enum) NewMovementMode "MOVE_Falling")
    (Class|XXIICharacter|EndDash)))

(event Input|MouseEvents|DebugKeyMouseWheelAxis
  (params (Key :type Key%20Structure :default "None") (ActionValue :type Input%20Action%20Value%20Structure))
  (bind _zoombounds (Variables|Zoom|GetZoomBounds))
  (:Pressed
    (if (and (!= (.x ActionValue) 0.0) (not (Audio|Components|Audio|IsPlaying (Variables|Default|GetZoom))))
      (Variables|Zoom|SetZoomMultiplier (Math|Float|Clamp(Float) (+ (Variables|Zoom|GetZoomMultiplier) (* (.x ActionValue) -1.0)) (.x _zoombounds) (.y _zoombounds))))))

(fn ConstructionScript
  (|CallParentFunction))

(fn UpdateCameraZoom
  (Variables|/Script/Engine.SpringArmComponent|SetTargetArmLength (Variables|Default|GetSpringArm) (Math|Interpolation|FInterpTo (Variables|/Script/Engine.SpringArmComponent|GetTargetArmLength (Variables|Default|GetSpringArm)) (* (Variables|Zoom|GetZoomMultiplier) (Variables|Zoom|GetZoomStep)) (Utilities|Time|GetWorldDeltaSeconds) 2.0)))

(fn SetPlayerSaveInformation
  (bind _savegame (Class|BPISaveGame|GetSelectedGameData(Message) (Game|GetGameInstance)))
  (bind _output_get (LocalVariables|SetSave _savegame))
  (Utilities|IsValid _output_get
    (:Is%20Valid
      (Utilities|FlowControl|Sequence
        (:then_0
          (bind _returnvalue (Game|GetCurrentLevelName true))
          (if (Utilities|Enum|Equal(Enum) (Variables|/Game/XXII/Core/SaveGame/BP_XXIISaveGame.BP_XXIISaveGame_C|GetSavedLevel (LocalVariables|GetSave)) _returnvalue)
            (if (not (== (Utilities|Struct|BreakFPlayerSave (Variables|/Game/XXII/Core/SaveGame/BP_XXIISaveGame.BP_XXIISaveGame_C|GetPlayerSave (LocalVariables|GetSave))) (Math|Transform|MakeTransform "0, 0, 0")))
              (Transformation|SetActorTransform (Utilities|Struct|BreakFPlayerSave (Variables|/Game/XXII/Core/SaveGame/BP_XXIISaveGame.BP_XXIISaveGame_C|GetPlayerSave (LocalVariables|GetSave)))))))
        (:then_1
          (if (not (CallFunction|IsStatDefault (Utilities|Struct|BreakFPlayerSave (Variables|/Game/XXII/Core/SaveGame/BP_XXIISaveGame.BP_XXIISaveGame_C|GetPlayerSave (LocalVariables|GetSave)))))
            (Variables|/Game/XXII/Core/Stat/BP_StatComponent.BP_StatComponent_C|SetStat (Variables|Default|GetStat%20Component) (Utilities|Struct|BreakFPlayerSave (Variables|/Game/XXII/Core/SaveGame/BP_XXIISaveGame.BP_XXIISaveGame_C|GetPlayerSave (LocalVariables|GetSave))))))))))