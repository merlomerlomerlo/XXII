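; BP_BaseCharacter is a base character Blueprint that exposes stats and tracks attack hits.
; Stat interface events for healing, damage and stamina use forward to PlayerStatComponent, as do stat queries and conditional stamina consumption.
; Both stamina consumption paths request a recharge start.
; CharacterAttackHit increments a capped hit count and, only when it changes, calls OnAttackHit with the raw and normalized count.
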(event EventHeal
  (params (HealAmount :type Float%20%28single-precision%29))
  ;[0.15 0.15 0.15 0.5] Stat Interface
  (Default|Heal (Variables|Default|GetPlayer%20Stat%20Component) HealAmount))

(event EventDamage
  (params (DamageAmount :type Float%20%28single-precision%29))
  ;[0.15 0.15 0.15 0.5] Stat Interface
  (Default|Damage (Variables|Default|GetPlayer%20Stat%20Component) DamageAmount))

(event EventConsumeStamina
  (params (StaminaAmount :type Float%20%28single-precision%29))
  ;[0.15 0.15 0.15 0.5] Stat Interface
  (Default|ConsumeStamina (Variables|Default|GetPlayer%20Stat%20Component) StaminaAmount true))

(fn ConstructionScript)

(fn GetStat
  (bind _player_stat_component (Variables|Default|GetPlayer%20Stat%20Component))
  (return (Utilities|Struct|MakeObjectStat (Variables|/Script/XXII.StatComponent|GetMaxHP _player_stat_component) (Variables|/Script/XXII.StatComponent|GetHP _player_stat_component) (Variables|/Script/XXII.StatComponent|GetMaxStaminaSegments _player_stat_component) (Variables|/Script/XXII.StatComponent|GetStamina _player_stat_component) (Variables|/Script/XXII.StatComponent|GetAttack _player_stat_component) (Variables|/Script/XXII.StatComponent|GetSpeed _player_stat_component))))

(fn TryConsumeStamina
  (params (StaminaAmount :type Float%20%28single-precision%29))
  (bind _result (Default|TryConsumeStamina (Variables|Default|GetPlayer%20Stat%20Component) StaminaAmount true))
  (return _result))

(fn CharacterAttackHit
  (if (!= (Math|Integer|Min(Integer) (+ (Variables|Character|GetHitCount) 1) (Variables|Character|GetMaxHitCount)) (Variables|Character|GetHitCount))
    (bind _output_get (Variables|Character|SetHitCount (Math|Integer|Min(Integer) (+ (Variables|Character|GetHitCount) 1) (Variables|Character|GetMaxHitCount))))
    (Default|CallOnAttackHit _output_get (/ _output_get (Variables|Character|GetMaxHitCount)))))