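; BP_BaseEnemy is a base enemy character that handles montage-driven attacks and death.
; Attack events play the montage mapped to the current or given stage, running a fast looping timer during playback, with an empty TraceAttack event alongside.
; Montage completion or interruption clears the timer and signals that the attack finished.
; The stat component's OnDeath disables capsule collision and sets a lifespan for removal.
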(event OnDeath(EnemyStatComponent)
  (Stat|HP|OnEnemyDeath))

(event Custom|TraceAttack)

(event Custom|StartAttack
  (bind _returnvalue (Utilities|Time|SetTimerbyEvent (EventDispatchers|CreateEvent :!event Custom|TraceAttack) 0.1 true)))

(event Custom|EndAttack
  (Utilities|Time|ClearandInvalidateTimerbyHandle (stale Custom|StartAttack _returnvalue))
  (Default|CallOnFinishAttack))

(event EventAttack
  (bind _stageattackmap (Variables|Enemy|Attack|GetStageAttackMap))
  (bind _currentstage (Variables|Enemy|Attack|GetCurrentStage))
  (bind _output (Utilities|Array|Get(acopy) _stageattackmap _currentstage))
  (Utilities|IsValid _output
    (:Is%20Valid
      (Animation|Montage|PlayMontage (Variables|Character|GetMesh) _output
        (:then
          (CallFunction|StartAttack))
        (:OnCompleted
          (CallFunction|EndAttack :!label _label))
        (:OnInterrupted
          (goto _label))))))

(event EventStageAttack
  (params (EnemyStage :type Integer))
  (bind _stageattackmap (Variables|Enemy|Attack|GetStageAttackMap))
  (bind _output (Utilities|Array|Get(acopy) _stageattackmap EnemyStage))
  (Utilities|IsValid _output
    (:Is%20Valid
      (Animation|Montage|PlayMontage (Variables|Character|GetMesh) _output
        (:then
          (CallFunction|StartAttack))
        (:OnCompleted
          (CallFunction|EndAttack :!label _label))
        (:OnInterrupted
          (goto _label))))))

(fn ConstructionScript
  (|CallParentFunction))

(fn OnEnemyDeath
  (Collision|SetCollisionEnabled (Variables|Default|GetCapsuleComponent) "NoCollision")
  (Actor|SetLifeSpan (Variables|Stat|HP|GetLifespanOnDeath)))