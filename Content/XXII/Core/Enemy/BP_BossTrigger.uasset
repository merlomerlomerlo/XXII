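; BP_BossTrigger is a gate that starts the fight with its referenced Boss and seals the way behind the player.
; When the player pawn ends overlap on the positive world-Y side of the Arrow, it pushes the boss HUD and calls StartBoss.
; The trigger then switches to BlockAll collision as a barrier.
; It binds to the Boss's OnDestroyed event, apparently to destroy itself and reopen the passage.
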(event OnComponentEndOverlap(BossTrigger)
  (params (OverlappedComponent :type Primitive%20Component%20Object%20Reference) (OtherActor :type Actor%20Object%20Reference) (OtherComp :type Primitive%20Component%20Object%20Reference) (OtherBodyIndex :type Integer))
  (if (== OtherActor (Game|Player|GetPlayerPawn 0))
    (if (> (.Y (Math|Vector|BreakVector (Math|Vector|GetUnitDirection(Vector) (Transformation|GetWorldLocation (Variables|Default|GetArrow)) (Transformation|GetActorLocation (Game|Player|GetPlayerPawn 0))))) 0.0)
      (CallFunction|OnBossStart))))

(event Custom|OnBossStart
  (Utilities|FlowControl|Sequence
    (:then_0
      (Variables|Boss|GetBoss
        (:then
          (bind _asbp_xxiihud (Utilities|Casting|CastToBP_XXIIHUD (HUD|GetHUD (Game|GetPlayerController 0))))
          (Default|PushBossHUD _asbp_xxiihud (Variables|Boss|GetBoss)))
        (:else)))
    (:then_1
      (Collision|SetCollisionProfileName (Variables|Default|GetBossTrigger) "BlockAll" true :!class /Script/Engine.PrimitiveComponent)
      (bind _boss (Variables|Boss|GetBoss)
        (:then
          (Default|StartBoss _boss))
        (:else)))))

(event Custom|OnBossDestroyed
  (params (DestroyedActor :type Actor%20Object%20Reference))
  (Actor|DestroyActor))

(event EventBeginPlay
  (bind _boss (Variables|Boss|GetBoss)
    (:then
      (Game|BindEventtoOnDestroyed _boss (EventDispatchers|CreateEvent :!event Custom|OnBossDestroyed)))
    (:else)))

(fn ConstructionScript)