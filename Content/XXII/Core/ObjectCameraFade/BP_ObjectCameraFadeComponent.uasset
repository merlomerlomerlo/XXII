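; Actor component that fades static mesh objects standing between the player camera and its owner.
; A looping timer started on BeginPlay drives WallFade, which multi-line traces from camera to owner and tracks hit actors in current and previous lists.
; FadeObject toggles the "Clip" scalar material parameter on each actor's static mesh component.
; When the trace finds nothing, a DoOnce, re-armed by hits, restores tracked objects and clears both lists.
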(event Custom|WallFade
  (bind (_outhits _returnvalue) (Collision|MultiLineTraceByChannel (Camera|GetCameraLocation (Game|GetPlayerCameraManager 0)) (Transformation|GetActorLocation (Components|GetOwner)) "TraceTypeQuery3" false 0 "None"))
  (if _returnvalue
    (for _array_element _outhits
      (bind _output_get (Variables|Default|SetCurrentObjectFade (.HitActor (Collision|BreakHitResult _array_element))))
      (if (and (not (Utilities|Array|ContainsItem (Variables|Default|GetObjectFade) _output_get)) (Utilities|IsValid (Actor|GetComponentbyClass _output_get "/Script/Engine.StaticMeshComponent")))
        (Utilities|Array|AddUnique (Variables|Default|GetObjectFade) (Variables|Default|GetCurrentObjectFade))
        (for _array_element_2 (Variables|Default|GetObjectFade)
          (CallFunction|FadeObject _array_element_2 true))
        (for _array_element_3 (Variables|Default|GetPreviousObjectFade)
          (CallFunction|FadeObject _array_element_3 false)
          (Utilities|Array|RemoveItem (Variables|Default|GetObjectFade) _array_element_3))
        (else
          (Variables|Default|SetPreviousObjectFade (Variables|Default|GetObjectFade)))))
    (CallFunction|ResetonTraceLost)
    (else
      (Utilities|FlowControl|DoOnce false
        (:Completed
          (for _array_element_4 (Variables|Default|GetObjectFade)
            (CallFunction|FadeObject _array_element_4 false))
          (Utilities|Array|Clear (Variables|Default|GetObjectFade))
          (Utilities|Array|Clear (Variables|Default|GetPreviousObjectFade)))))))

(event Custom|ResetOnTraceLost
  (Utilities|FlowControl|DoOnce false) ; enters at Reset
)

(event EventBeginPlay
  (Utilities|Time|SetTimerbyEvent (EventDispatchers|CreateEvent :!event Custom|WallFade) 0.1 true))

(fn FadeObject
  (params (ObjectToFade :type Actor%20Object%20Reference) (ClipWall :type Boolean))
  (bind _returnvalue (Actor|GetComponentbyClass ObjectToFade "/Script/Engine.StaticMeshComponent"))
  (Utilities|IsValid _returnvalue
    (:Is%20Valid
      (Rendering|Material|SetScalarParameterValueonMaterials _returnvalue "Clip" (Math|Conversions|ToFloat(Boolean) ClipWall)))))