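; Player stat component, derived from a parent stat class, that manages HP and stamina and sets the owning character's walk speed on BeginPlay.
; Looping timers drive delayed stamina recharge and periodic drain, each stopping the other, while TryConsumeStamina permits spending whenever any stamina remains.
; Refreshing max stamina refills instantly or starts recharge when neither timer runs.
; Heal and Damage clamp HP and broadcast changes, though Damage skips the broadcast at zero.
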(event Custom|StaminaRecharge
  ;[0.15 0.15 0.15 0.5] Stamina Recharge
  (bind _result (Utilities|+=(Float) (Variables|Default|GetStamina) (Variables|Stat|Stamina|GetStaminaRechargeAmount)))
  (bind _output_get (Variables|Default|SetStamina (Math|Float|Min(Float) _result (Variables|Default|GetCurrentMaxStamina))))
  (Default|CallOnChangeStamina _output_get (/ _output_get (Variables|Default|GetCurrentMaxStamina)))
  (if (>= (Variables|Default|GetStamina) (Variables|Default|GetCurrentMaxStamina))
    (CallFunction|StopStaminaRecharge)))

(event Custom|StartStaminaRecharge
  ;[0.15 0.15 0.15 0.5] Stamina Recharge
  (CallFunction|StopStaminaRecharge)
  (Variables|Default|SetbIsRecharging true)
  (bind _returnvalue (Utilities|Time|SetTimerbyEvent (EventDispatchers|CreateEvent :!event Custom|StaminaRecharge) (Variables|Stat|Stamina|GetStaminaRechargeFrequence) true true (Variables|Stat|Stamina|GetStaminaRechargeDelay)))
  (Variables|Stat|Stamina|Handle|SetStaminaRechargeHandle _returnvalue))

(event Custom|StopStaminaRecharge
  ;[0.15 0.15 0.15 0.5] Stamina Recharge
  (Utilities|Time|ClearandInvalidateTimerbyHandle (Variables|Stat|Stamina|Handle|GetStaminaRechargeHandle))
  (Variables|Default|SetbIsRecharging false))

(event Custom|StaminaConsumePerFrequency_Tick
  ;[0.15 0.15 0.15 0.5] Stamina Recharge
  ;;[0.05729 0.05729 0.05729 0.5] Stamina Consume per frequency handle
  (bind _result (Stat|Stamina|TryConsumeStamina (stale Custom|StartStaminaConsume StaminaConsumeAmount) false))
  (if (not _result)
    (CallFunction|StopStaminaConsume)))

(event Custom|StartStaminaConsume
  (params (StaminaConsumeFrequency :type Float%20%28double-precision%29) (StaminaConsumeAmount :type Float%20%28double-precision%29))
  ;[0.15 0.15 0.15 0.5] Stamina Recharge
  ;;[0.05729 0.05729 0.05729 0.5] Stamina Consume per frequency handle
  (CallFunction|StopStaminaRecharge)
  (CallFunction|StopStaminaConsume)
  (bind _returnvalue (Utilities|Time|SetTimerbyEvent (EventDispatchers|CreateEvent :!event Custom|StaminaConsumePerFrequency_Tick) StaminaConsumeFrequency true true))
  (Variables|Stat|Stamina|Handle|SetStaminaConsumePerFrequency _returnvalue)
  (Variables|Default|SetbIsConsuming true))

(event Custom|StopStaminaConsume
  ;[0.15 0.15 0.15 0.5] Stamina Recharge
  ;;[0.05729 0.05729 0.05729 0.5] Stamina Consume per frequency handle
  (Utilities|Time|ClearandInvalidateTimerbyHandle (Variables|Stat|Stamina|Handle|GetStaminaConsumePerFrequency))
  (CallFunction|StartStaminaRecharge)
  (Variables|Default|SetbIsConsuming false))

(event EventBeginPlay
  (|CallParentFunction)
  (bind _ascharacter (Utilities|Casting|CastToCharacter (Components|GetOwner)))
  (bind _charactermovement (Variables|/Script/Engine.Character|GetCharacterMovement _ascharacter)
    (:then
      (Variables|/Script/Engine.CharacterMovementComponent|SetMaxWalkSpeed _charactermovement (Variables|Stat|Action|Locomotion|GetWalkSpeed)))
    (:else)))

(event EventRefreshCurrentMaxStamina
  ;[0.15 0.15 0.15 0.5] Stamina Refresh on change HP
  (|CallParentFunction)
  (if (and (not (Utilities|Time|IsTimerActivebyHandle (Variables|Stat|Stamina|Handle|GetStaminaRechargeHandle))) (not (Utilities|Time|IsTimerActivebyHandle (Variables|Stat|Stamina|Handle|GetStaminaConsumePerFrequency))))
    (if (Variables|Stat|Debug|GetInstantStaminaRecharge)
      (bind _output_get (Variables|Default|SetStamina (Variables|Default|GetCurrentMaxStamina)))
      (Default|CallOnChangeStamina _output_get 1.0)
      (else
        (CallFunction|StartStaminaRecharge)))))

(event EventTick
  (params (DeltaSeconds :type Float%20%28single-precision%29))
  (Stat|Debug|DebugStat))

(fn DebugStat
  (if (Variables|Stat|Debug|GetDebugStats)
    (Utilities|FlowControl|Sequence
      (:then_0
        (Development|PrintString (Utilities|String|Append "Stamina: " (Utilities|String|ToString(Float) (Variables|Default|GetStamina))) true false "(R=1.000000,G=0.306726,B=0.000000,A=1.000000)" 0.1 "StatStamina"))
      (:then_1
        (Development|PrintString (Utilities|String|Append "HP: " (Utilities|String|ToString(Float) (Variables|Default|GetHP))) true false "(R=0.236897,G=1.000000,B=0.083865,A=1.000000)" 0.1 "StatHP"))
      (:then_2
        (Development|PrintString (Utilities|String|Append (Utilities|GetDisplayName (Components|GetOwner)) " Stat:") true false "(R=0.886886,G=0.028134,B=1.000000,A=1.000000)" 0.1 "StatHeader")))))

(fn Heal
  (params (HealAmount :type Float%20%28double-precision%29))
  (bind _output_get (Variables|Default|SetHP (Math|Float|Min(Float) (+ (Variables|Default|GetHP) (Math|Float|Absolute(Float) HealAmount)) (Variables|Default|GetMaxHP))))
  (Default|CallOnChangeHP _output_get (/ _output_get (Variables|Default|GetMaxHP))))

(fn Damage
  (params (DamageAmount :type Float%20%28double-precision%29))
  (bind _output_get (Variables|Default|SetHP (Math|Float|Max(Float) (- (Variables|Default|GetHP) (Math|Float|Absolute(Float) DamageAmount)) 0.0)))
  (if (> _output_get 0.0)
    (Default|CallOnChangeHP (Variables|Default|GetHP) (/ (Variables|Default|GetHP) (Variables|Default|GetMaxHP)))))

(fn CanDoAction
  (params (StaminaAmount :type Float%20%28double-precision%29))
  (return (> (Variables|Default|GetStamina) 0.0)))

(fn ConsumeStamina
  (params (StaminaAmount :type Float%20%28double-precision%29) (StartRecharge :type Boolean))
  (Utilities|FlowControl|Sequence
    (:then_0
      (if (Utilities|Time|IsTimerActivebyHandle (Variables|Stat|Stamina|Handle|GetStaminaRechargeHandle))
        (CallFunction|StopStaminaRecharge)))
    (:then_1
      (bind _output_get (Variables|Default|SetStamina (Math|Float|Max(Float) (- (Variables|Default|GetStamina) StaminaAmount) 0.0)))
      (Default|CallOnChangeStamina _output_get (/ _output_get (Variables|Default|GetCurrentMaxStamina)))
      (if StartRecharge
        (CallFunction|StartStaminaRecharge)
        (return)))))

(fn TryConsumeStamina
  (params (StaminaAmount :type Float%20%28double-precision%29) (StartRecharge :type Boolean))
  (if (Stat|Stamina|CanDoAction StaminaAmount)
    (Stat|Stamina|ConsumeStamina StaminaAmount StartRecharge)
    (return true)
    (else
      (return false))))

(fn IsRechargingStamina
  (return (Variables|Default|GetbIsRecharging)))

(fn IsConsumingStamina
  (return (Variables|Default|GetbIsConsuming)))