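; Stat component that manages an FPlayerStat struct and fires OnDeath when checked HP is at or below zero.
; Damage and Heal adjust HP by absolute amounts with no clamping, then run the death check, as does SetStat.
; SetStat applies Min against zero to HP, Stamina, Attack and Speed, capping them at zero rather than flooring them.
; IncreaseMaxHP and DecreaseMaxHP both add the absolute amount through SetMaxHP.
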(event EventBeginPlay)

(fn SetStat
  (params (Stat :type F%20Player%20Stat%20Structure))
  (bind (_hp _stamina _attack _speed) (Utilities|Struct|BreakFPlayerStat Stat))
  (bind _structout (Utilities|Struct|SetmembersinFPlayerStat (Variables|StatComponent|GetStat) (Math|Float|Min(Float) _hp 0.0) (Math|Float|Min(Float) _stamina 0.0) (Math|Float|Min(Float) _attack 0.0) (Math|Float|Min(Float) _speed 0.0)))
  (StatComponent|HP|CheckonDeath (Utilities|Struct|BreakFPlayerStat _structout)))

(fn CheckonDeath
  (params (HP :type Float%20%28double-precision%29))
  (if (<= HP 0.0)
    (Default|CallOnDeath)))

(fn Damage
  (params (DamageAmount :type Float%20%28double-precision%29))
  (bind _structout (Utilities|Struct|SetmembersinFPlayerStat (Variables|StatComponent|GetStat) (- (Utilities|Struct|BreakFPlayerStat (Variables|StatComponent|GetStat)) (Math|Float|Absolute(Float) DamageAmount))))
  (StatComponent|HP|CheckonDeath (Utilities|Struct|BreakFPlayerStat _structout)))

(fn Heal
  (params (HealAmount :type Float%20%28double-precision%29))
  (bind _structout (Utilities|Struct|SetmembersinFPlayerStat (Variables|StatComponent|GetStat) (+ (Utilities|Struct|BreakFPlayerStat (Variables|StatComponent|GetStat)) (Math|Float|Absolute(Float) HealAmount))))
  (StatComponent|HP|CheckonDeath (Utilities|Struct|BreakFPlayerStat _structout)))

(fn SetMaxHP
  (params (MaxHP :type Float%20%28double-precision%29))
  (Utilities|Struct|SetmembersinFPlayerStat (Variables|StatComponent|GetStat) MaxHP))

(fn IncreaseMaxHP
  (params (IncreaseAmount :type Float%20%28double-precision%29))
  (StatComponent|HP|SetMaxHP (+ (Utilities|Struct|BreakFPlayerStat (Variables|StatComponent|GetStat)) (Math|Float|Absolute(Float) IncreaseAmount))))

(fn DecreaseMaxHP
  (params (DecreaseAmount :type Float%20%28double-precision%29))
  (StatComponent|HP|SetMaxHP (+ (Utilities|Struct|BreakFPlayerStat (Variables|StatComponent|GetStat)) (Math|Float|Absolute(Float) DecreaseAmount))))