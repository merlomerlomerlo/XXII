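; Papercutter weapon actor whose blade pieces act as a health display, with one piece visible per point of player HP.
; On BeginPlay it gathers root child components named "piece" and inserts them into SwordPieces by their two-digit name suffix.
; It binds to the HP change event on player 0's BP_StatComponent, showing pieces with an index below current HP and hiding the rest.
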(event Custom|OnPlayerDamage
  (params (CurrentHP :type Float%20%28double-precision%29))
  (bind (_arrayindex _arrayelement) (Utilities|Array|ReverseforEachLoop (Variables|Default|GetSwordPieces))
    (:LoopBody
      (Rendering|SetVisibility _arrayelement (> CurrentHP _arrayindex) false))))

(event EventBeginPlay
  (Utilities|FlowControl|Sequence
    (:then_0
      (Utilities|Array|Clear (Variables|Default|GetSwordPieces))
      (for _array_element (Components|GetChildrenComponents (Variables|Default|GetDefaultSceneRoot) false)
        (if (Utilities|String|Contains (Utilities|String|ToLower (Utilities|GetDisplayName _array_element)) "piece" false true)
          (Utilities|Array|Insert (Variables|Default|GetSwordPieces) _array_element (- (Math|Conversions|ToInteger(Byte) (Utilities|String|Right (Utilities|GetDisplayName _array_element) 2)) 1)))))
    (:then_1
      (bind _returnvalue (Actor|GetComponentbyClass (Game|Player|GetPlayerPawn 0) "/Game/XXII/Core/Stat/BP_StatComponent.BP_StatComponent_C"))
      (Utilities|IsValid _returnvalue
        (:Is%20Valid
          (EventDispatchers|BindEventtoOnChangeHP _returnvalue (EventDispatchers|CreateEvent :!event Custom|OnPlayerDamage)))))))

(fn ConstructionScript)