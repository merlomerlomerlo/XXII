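; Checkpoint actor that saves game progress when the player pawn enters its sphere trigger.
; On overlap it sends the game instance three save messages: the current time, the current level name, and player data.
; The player data struct combines the pawn's transform with stats fetched from the pawn through a message call, so the checkpoint needs no casts.
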(event OnComponentBeginOverlap(Sphere)
  (params (OverlappedComponent :type Primitive%20Component%20Object%20Reference) (OtherActor :type Actor%20Object%20Reference) (OtherComp :type Primitive%20Component%20Object%20Reference) (OtherBodyIndex :type Integer) (bFromSweep :type Boolean) (SweepResult :type Hit%20Result%20Structure%20%28by%20ref%29))
  (bind _returnvalue (Game|Player|GetPlayerPawn 0))
  (if (== OtherActor (Game|Player|GetPlayerPawn 0))
    (Class|BPISaveGame|SaveGameInfoData(Message) (Game|GetGameInstance) (Math|DateTime|Now))
    (bind _returnvalue_2 (Game|GetCurrentLevelName true))
    (Class|BPISaveGame|SaveMapData(Message) (Game|GetGameInstance) _returnvalue_2)
    (bind _returnvalue_3 (Class|StatInterface|GetStat(Message) _returnvalue))
    (Class|BPISaveGame|SavePlayerData(Message) (Game|GetGameInstance) (Utilities|Struct|MakeFPlayerSave (Transformation|GetActorTransform _returnvalue) _returnvalue_3))))

(fn ConstructionScript)